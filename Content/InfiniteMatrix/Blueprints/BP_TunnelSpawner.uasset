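; BP_TunnelSpawner builds a chain of BP_Tunnel segments, apparently for an endless tunnel level.
; On BeginPlay it destroys existing tunnels, then spawns a short starting run from the player pawn's location.
; Each further segment spawns at the newest tunnel's SpawnPoint.
; Every new tunnel receives a reference back to the spawner and randomizes its wall, health pack and enemy.
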(event `self.ReceiveBeginPlay`
  (`self.SpawnInitialTunnels`))

(fn `SpawnInitialTunnels`
  (`|ExecutionSequence`
    (:`then_0`
      (bind _outactors (`GameplayStatics.GetAllActorsOfClass` "/Game/InfiniteMatrix/Blueprints/BP_Tunnel.BP_Tunnel_C"))
      (for _array_element _outactors
        (`self.K2_DestroyActor` _array_element)))
    (:`then_1`
      (for _ (range 3)
        (if (`KismetSystemLibrary.IsValid` (`self.NewestTunnel`))
          (`self.SpawnTunnelAtSpawnPoint`)
          (else
            (`self.SpawnNewTunnel` (`self.K2_GetActorLocation` (`GameplayStatics.GetPlayerPawn` 0)))))))))

(fn `SpawnNewTunnel`
  (params (NewParam :type "Vector Structure"))
  (bind _returnvalue (`|SpawnActorFromClass` "/Game/InfiniteMatrix/Blueprints/BP_Tunnel.BP_Tunnel_C" (`KismetMathLibrary.Conv_VectorToTransform` NewParam) "Undefined" "MultiplyWithRoot" null null))
  (bind _output_get (set `self.NewestTunnel` _returnvalue))
  (set `/Game/InfiniteMatrix/Blueprints/BP_Tunnel.TunnelSpawner` self _output_get)
  (`/Game/InfiniteMatrix/Blueprints/BP_Tunnel.RandomizeWall` _output_get)
  (`/Game/InfiniteMatrix/Blueprints/BP_Tunnel.RandomizeHealthPack` _output_get)
  (`/Game/InfiniteMatrix/Blueprints/BP_Tunnel.RandomizeEnemny` _output_get))

(fn `SpawnTunnelAtSpawnPoint`
  (`self.SpawnNewTunnel` (`SceneComponent.K2_GetComponentLocation` (`/Game/InfiniteMatrix/Blueprints/BP_Tunnel.SpawnPoint` (`self.NewestTunnel`)))))

(fn `UserConstructionScript`)