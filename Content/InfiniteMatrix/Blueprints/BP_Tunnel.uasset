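; BP_Tunnel is a tunnel segment with a rotating holed wall that damages BP_Player and destroys projectiles.
; Randomize functions choose the wall mesh and rotation, spawn a health pack and place enemies at shuffled points.
; Crossing TriggerZone adds speed-based score unless the wall was hit, asks TunnelSpawner for another segment, then removes the tunnel and its health pack.
; The enemy cleanup loop calls DestroyActor on the tunnel itself.
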(event `self.ReceiveBeginPlay`
  (bind _enemyspawnpositionset (`self.EnemySpawnPositionSet`))
  (bind _healthpackpositionset (`self.HealthPackPositionSet`))
  (`KismetArrayLibrary.Array_Set` _healthpackpositionset 0 (`self.HealthPackPosition1`))
  (`KismetArrayLibrary.Array_Set` _healthpackpositionset 1 (`self.HealthPackPosition2`))
  (`KismetArrayLibrary.Array_Set` _healthpackpositionset 2 (`self.HealthPackPosition3`))
  (`KismetArrayLibrary.Array_Set` _healthpackpositionset 3 (`self.HealthPackPosition4`))
  (`KismetArrayLibrary.Array_Set` _enemyspawnpositionset 0 (`self.EnemySpawnPostion`))
  (`KismetArrayLibrary.Array_Set` _enemyspawnpositionset 1 (`self.EnemySpawnPostion1`))
  (`KismetArrayLibrary.Array_Set` _enemyspawnpositionset 2 (`self.EnemySpawnPostion2`))
  (`KismetArrayLibrary.Array_Set` _enemyspawnpositionset 3 (`self.EnemySpawnPostion3`))
  (`KismetArrayLibrary.Array_Set` _enemyspawnpositionset 4 (`self.EnemySpawnPostion4`)))

(event `self.ReceiveTick`
  (params (DeltaSeconds :type "Float (single-precision)"))
  (`SceneComponent.K2_AddLocalRotation` (`self.WallMesh`) (`KismetMathLibrary.MakeRotator` (* DeltaSeconds (`self.RotateSpeed`))) false false))

(event `self.TriggerZone.OnComponentBeginOverlap`
  (params (OverlappedComponent :type "PrimitiveComponent Object Reference") (OtherActor :type "Actor Object Reference") (OtherComp :type "PrimitiveComponent Object Reference") (OtherBodyIndex :type Integer) (bFromSweep :type Boolean) (SweepResult :type "HitResult Structure (by ref)"))
  (bind _healthpacklocal (`self.HealthPackLocal`))
  (bind _asbp_player (cast `/Game/InfiniteMatrix/Blueprints/BP_Player` OtherActor))
  (if (not (`self.IfHit`))
    (set `/Game/InfiniteMatrix/Blueprints/BP_Player.Score` (+ (`/Game/InfiniteMatrix/Blueprints/BP_Player.Score` _asbp_player) (/ (`/Game/InfiniteMatrix/Blueprints/BP_Player.MoveSpeed` _asbp_player) 200.0)) _asbp_player))
  (set `self.IfHit` false)
  (`/Game/InfiniteMatrix/Blueprints/BP_TunnelSpawner.SpawnTunnelAtSpawnPoint` (`self.TunnelSpawner`))
  (`/Engine/EditorBlueprintResources/StandardMacros.IsValid` _healthpacklocal
    (:`Is Valid`
      (`self.K2_DestroyActor` _healthpacklocal))
    (:`Is Not Valid`
      _))
  (for _index (range 5)
    (`/Engine/EditorBlueprintResources/StandardMacros.IsValid` (`|GetArrayItem` (`self.EnemyLocal`) _index)
      (:`Is Valid`
        (`KismetSystemLibrary.PrintString` "Delete")
        (`self.K2_DestroyActor`))))
  (`self.K2_DestroyActor`))

(event `self.WallMesh.OnComponentBeginOverlap`
  (params (OverlappedComponent :type "PrimitiveComponent Object Reference") (OtherActor :type "Actor Object Reference") (OtherComp :type "PrimitiveComponent Object Reference") (OtherBodyIndex :type Integer) (bFromSweep :type Boolean) (SweepResult :type "HitResult Structure (by ref)"))
  (set `self.IfHit` true)
  (bind _asbp_player (cast `/Game/InfiniteMatrix/Blueprints/BP_Player` OtherActor)
    (:`then`
      (`/Game/InfiniteMatrix/Blueprints/BP_Player.LoseHealth` _asbp_player 30))
    (:`CastFailed`
      (bind _asbp_projectile (cast `/Game/InfiniteMatrix/Blueprints/BP_Projectile` OtherActor))
      (`self.K2_DestroyActor` _asbp_projectile))))

(fn `RandomizeEnemny`
  (bind _output_get (set `self.EnemySpawnPositionSetCopy` (`self.EnemySpawnPositionSet`)))
  (`KismetArrayLibrary.Array_Shuffle` _output_get)
  (for (_array_element _array_index) _output_get
    (if (not (> _array_index (`KismetMathLibrary.RandomIntegerInRange` 0 4)))
      (bind _returnvalue (`|SpawnActorFromClass` "/Game/InfiniteMatrix/Blueprints/BP_Enemy.BP_Enemy_C" (`KismetMathLibrary.Conv_VectorToTransform` (`SceneComponent.K2_GetComponentLocation` _array_element)) "Undefined" "MultiplyWithRoot" null null))
      (`KismetArrayLibrary.Array_Set` (`self.EnemyLocal`) _array_index _returnvalue))))

(fn `RandomizeHealthPack`
  (bind _returnvalue (`|SpawnActorFromClass` "/Game/InfiniteMatrix/Blueprints/BP_HealthPack.BP_HealthPack_C" (`KismetMathLibrary.Conv_VectorToTransform` (`SceneComponent.K2_GetComponentLocation` (`|GetArrayItem` (`self.HealthPackPositionSet`) (`KismetMathLibrary.RandomIntegerInRange` 0 3)))) "Undefined" "MultiplyWithRoot" null null))
  (bind _output_get (set `self.HealthPackLocal` _returnvalue))
  (`SceneComponent.K2_AddLocalRotation` (`Actor.RootComponent` _output_get) (`KismetMathLibrary.MakeRotator` 0.0 0.0 (`KismetMathLibrary.RandomFloatInRange` 0.0 360.0)) false false))

(fn `RandomizeWall`
  (`StaticMeshComponent.SetStaticMesh` (`self.WallMesh`) (select `int` (`KismetMathLibrary.RandomIntegerInRange` 0 3) :`0` "/Game/InfiniteMatrix/Meshes/SM_Hole_01.SM_Hole_01" :`1` "/Game/InfiniteMatrix/Meshes/SM_Hole_02.SM_Hole_02" :`2` "/Game/InfiniteMatrix/Meshes/SM_Hole_03.SM_Hole_03" :`3` "/Game/InfiniteMatrix/Meshes/SM_Hole_04.SM_Hole_04" :!type "StaticMesh Object Reference"))
  (`SceneComponent.K2_AddLocalRotation` (`self.WallMesh`) (`KismetMathLibrary.MakeRotator` (`KismetMathLibrary.RandomFloatInRange` 0.0 360.0)) false false))

(fn `UserConstructionScript`)